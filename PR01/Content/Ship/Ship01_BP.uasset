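; Ship Blueprint that handles player axis input for an orbit-style camera and thruster-driven roll.
; Yaw input rotates an azimuth gimbal and pitch input rotates the spring arm, while zoom incrementally changes arm length from a stored value, all scaled by delta time.
; Roll input activates the left and right wing thrust components and sets both to the same axis-scaled RollStrength.
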(event `self.ReceiveBeginPlay`
  (set `self.SpringArmDefault` (`SpringArmComponent.TargetArmLength` (`self.SpringArm`))))

(event `InputAxis|AimZoom`
  (params (AxisValue :type "Float (single-precision)"))
  ;[1 1 1] Zoom
  (bind _output_get (set `SpringArmComponent.TargetArmLength` (+ (* AxisValue (`GameplayStatics.GetWorldDeltaSeconds`) 1000.0) (`self.SpringArmDefault`)) (`self.SpringArm`)))
  (set `self.SpringArmDefault` _output_get))

(event `InputAxis|AimRoll`
  (params (AxisValue :type "Float (single-precision)"))
  (bind _leftwingrollthrust (`self.LeftWingRollThrust`))
  (bind _rightwingrollthrust (`self.RightWingRollThrust`))
  (bind _returnvalue (* AxisValue (`self.RollStrength`)))
  (`ActorComponent.Activate` _leftwingrollthrust false)
  (`ActorComponent.Activate` _rightwingrollthrust false)
  (set `PhysicsThrusterComponent.ThrustStrength` _returnvalue _leftwingrollthrust)
  (set `PhysicsThrusterComponent.ThrustStrength` _returnvalue _rightwingrollthrust))

(event `InputAxis|AimYaw`
  (params (AxisValue :type "Float (single-precision)"))
  ;[1 1 1] Yaw
  (`SceneComponent.K2_AddLocalRotation` (`self.AzumutGimbal`) (`KismetMathLibrary.MakeRotator` 0.0 0.0 (* AxisValue (`GameplayStatics.GetWorldDeltaSeconds`) 100.0)) false false))

(event `InputAxis|AimPitch`
  (params (AxisValue :type "Float (single-precision)"))
  ;[1 1 1] Pitch
  (`SceneComponent.K2_AddLocalRotation` (`self.SpringArm`) (`KismetMathLibrary.MakeRotator` 0.0 (* AxisValue (`GameplayStatics.GetWorldDeltaSeconds`) 100.0)) false false))

(fn `UserConstructionScript`)